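; Trigger box that shows the ApuñalaTutorial (stab) widget when the FirstPersonCharacter enters it, if tutorials are enabled in the GlobalVariables game instance.
; Begin overlap creates the widget, shows the cursor, disables character input and flags the tutorial as active, with a counter blocking duplicates.
; End overlap removes the widget, restores input and cursor, and resets the counter, so re-entry can show it again.
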(event OnComponentBeginOverlap(CollisionComponent)
  (params (OverlappedComponent :type Primitive%20Component%20Object%20Reference) (OtherActor :type Actor%20Object%20Reference) (OtherComp :type Primitive%20Component%20Object%20Reference) (OtherBodyIndex :type Integer) (bFromSweep :type Boolean) (SweepResult :type Hit%20Result%20Structure%20%28by%20ref%29))
  (Utilities|Casting|CastToFirstPersonCharacter OtherActor)
  (bind _asglobal_variables (Utilities|Casting|CastToGlobalVariables (Game|GetGameInstance)))
  (if (Variables|/Game/FirstPersonBP/GlobalVariables.GlobalVariables_C|GetTutorialEncendido _asglobal_variables)
    (if (== (Variables|Default|GetContador) 0)
      (Variables|Default|SetContador 1)
      (bind _returnvalue (UserInterface|CreateWidget "/Game/Widgets/TutorialWidget/Apuñala-TutorialWidget.Apuñala-TutorialWidget_C"))
      (Variables|/Script/Engine.PlayerController|SetbShowMouseCursor (Game|GetPlayerController 0) true)
      (Input|DisableInput (Game|GetPlayerCharacter 0) (Game|GetPlayerController 0))
      (UserInterface|Viewport|AddtoViewport _returnvalue 0)
      (Variables|/Game/FirstPersonBP/GlobalVariables.GlobalVariables_C|SetApuñalaTutorialEncendido _asglobal_variables true)
      (Variables|Default|SetOverlapped true))))

(event OnComponentEndOverlap(CollisionComponent)
  (params (OverlappedComponent :type Primitive%20Component%20Object%20Reference) (OtherActor :type Actor%20Object%20Reference) (OtherComp :type Primitive%20Component%20Object%20Reference) (OtherBodyIndex :type Integer))
  (if (Variables|Default|GetOverlapped)
    (Utilities|Casting|CastToFirstPersonCharacter OtherActor)
    (bind _asglobal_variables (Utilities|Casting|CastToGlobalVariables (Game|GetGameInstance)))
    (if (Variables|/Game/FirstPersonBP/GlobalVariables.GlobalVariables_C|GetTutorialEncendido _asglobal_variables)
      (Variables|Default|SetContador 0)
      (Widget|RemovefromParent (stale OnComponentBeginOverlap(CollisionComponent) _returnvalue))
      (Variables|/Game/FirstPersonBP/GlobalVariables.GlobalVariables_C|SetApuñalaTutorialEncendido _asglobal_variables false)
      (Input|EnableInput (Game|GetPlayerCharacter 0) (Game|GetPlayerController 0))
      (Variables|/Script/Engine.PlayerController|SetbShowMouseCursor (Game|GetPlayerController 0) false))))

(event EventBeginPlay)

(event Collision|EventActorBeginOverlap
  (params (OtherActor :type Actor%20Object%20Reference)))

(event EventTick
  (params (DeltaSeconds :type Float%20%28single-precision%29)))

(fn ConstructionScript)