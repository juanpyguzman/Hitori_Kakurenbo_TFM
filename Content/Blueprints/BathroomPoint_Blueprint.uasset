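; BathroomPoint is a goal trigger actor that lets the player win, but only after the enemy has reached it first.
; It caches the first-person character on BeginPlay, then its collision component waits for the Enemy stored in the GlobalVariables game instance to overlap and set PlayerTurn.
; Once that flag is set, a player overlap sets PlayerWon on the game instance and calls PlayerVictory on the character.
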(event OnComponentBeginOverlap(CollisionComponent)
  (params (OverlappedComponent :type Primitive%20Component%20Object%20Reference) (OtherActor :type Actor%20Object%20Reference) (OtherComp :type Primitive%20Component%20Object%20Reference) (OtherBodyIndex :type Integer) (bFromSweep :type Boolean) (SweepResult :type Hit%20Result%20Structure%20%28by%20ref%29))
  (if (Variables|Default|GetPlayerTurn)
    (if (== OtherActor (Variables|Default|GetPlayer))
      (bind _asglobal_variables (Utilities|Casting|CastToGlobalVariables (Game|GetGameInstance)))
      (Variables|/Game/FirstPersonBP/GlobalVariables.GlobalVariables_C|SetPlayerWon _asglobal_variables true)
      (Default|PlayerVictory (Variables|Default|GetPlayer)))
    (else
      (bind _asglobal_variables_2 (Utilities|Casting|CastToGlobalVariables (Game|GetGameInstance)))
      (if (== OtherActor (Variables|/Game/FirstPersonBP/GlobalVariables.GlobalVariables_C|GetEnemy _asglobal_variables_2))
        (Variables|Default|SetPlayerTurn true)))))

(event EventBeginPlay
  (bind _asfirst_person_character (Utilities|Casting|CastToFirstPersonCharacter (Game|GetPlayerCharacter 0)))
  (Variables|Default|SetPlayer _asfirst_person_character)
  (Variables|Default|SetPlayerTurn false))

(event Collision|EventActorBeginOverlap
  (params (OtherActor :type Actor%20Object%20Reference)))

(event EventTick
  (params (DeltaSeconds :type Float%20%28single-precision%29)))

(fn ConstructionScript)