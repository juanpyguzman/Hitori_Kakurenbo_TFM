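; Main bathroom door actor that either starts open during the tutorial or swings open on a timer tied to the enemy.
; On BeginPlay it reads the tutorial flag from the GlobalVariables game instance, snapping open or arming AbrirPuerta.
; While armed, Tick waits on a Delay one second shorter than the enemy AI controller's Countdown.
; It then runs a Timeline that drives relative yaw, clears the flag and plays an attenuated opening sound.
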(event Custom|Abrir%20Puerta
  (bind _angle (Timeline|Abrir_Puerta_Timelline Play)
    (:Update
      (Transformation|SetActorRelativeRotation (Math|Rotator|MakeRotator 0.0 0.0 (* _angle 1.6e+02))))))

(event EventBeginPlay
  (bind _asglobal_variables (Utilities|Casting|CastToGlobalVariables (Game|GetGameInstance)))
  (if (Variables|/Game/FirstPersonBP/GlobalVariables.GlobalVariables_C|GetTutorialEncendido _asglobal_variables)
    (Transformation|SetActorRelativeRotation (Math|Rotator|MakeRotator 0.0 0.0 1.6e+02))
    (else
      (Variables|Default|SetAbrirPuerta true))))

(event Collision|EventActorBeginOverlap
  (params (OtherActor :type Actor%20Object%20Reference)))

(event EventTick
  (params (DeltaSeconds :type Float%20%28single-precision%29))
  (bind _self self)
  (if (Variables|Default|GetAbrirPuerta)
    (bind _asglobal_variables (Utilities|Casting|CastToGlobalVariables (Game|GetGameInstance)))
    (bind _asbp_aicontroller_enemy_2 (Utilities|Casting|CastToBP_AIController_Enemy_2 (AI|GetAIController (Variables|/Game/FirstPersonBP/GlobalVariables.GlobalVariables_C|GetEnemy _asglobal_variables))))
    (Utilities|FlowControl|Delay (Math|Conversions|ToFloat(Integer) (- (Variables|/Game/Muñeco/IA/BP_AIController_Enemy_2.BP_AIController_Enemy_2_C|GetCountdown _asbp_aicontroller_enemy_2) 1)))
    (CallFunction|AbrirPuerta)
    (Variables|Default|SetAbrirPuerta false)
    (Audio|PlaySoundatLocation "/Game/Sounds/Effects/Door_Opening__Sound_Effect.Door_Opening__Sound_Effect" (Transformation|GetActorLocation _self) (Transformation|GetActorRotation _self) 0.2 1.0 0.0 "/Game/Sounds/Effects/Door_Opening_Attenuation.Door_Opening_Attenuation" 0 0)))

(fn ConstructionScript)