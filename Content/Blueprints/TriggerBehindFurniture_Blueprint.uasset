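; Hiding-spot trigger that lets the first-person player go prone under a car, out of AI sight.
; Overlap shows a Spanish prompt and opens a gate for the prone input, which removes the prompt, unregisters the player's sight stimulus and calls ProneEvent.
; Leaving re-registers sight, then either calls ProneEvent again if hidden or clears the prompt and closes the gate.
; Also pitches an inside camera within limits; unconnected leftover cupboard-exit logic remains.
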(event OnComponentEndOverlap(CollisionComponent)
  (params (OverlappedComponent :type Primitive%20Component%20Object%20Reference) (OtherActor :type Actor%20Object%20Reference) (OtherComp :type Primitive%20Component%20Object%20Reference) (OtherBodyIndex :type Integer))
  (bind _playercharacter (Variables|Default|GetPlayerCharacter))
  (bind _playercharacter_2 (Variables|Default|GetPlayerCharacter))
  (Utilities|Casting|CastToFirstPersonCharacter OtherActor)
  (Class|AIPerceptionStimuliSourceComponent|RegisterforSense (Variables|/Game/FirstPersonBP/Blueprints/FirstPersonCharacter.FirstPersonCharacter_C|GetAIPerceptionStimuliSource _playercharacter) "/Script/AIModule.AISense_Sight")
  (if (== (Variables|Default|GetContadorEntrada) 0)
    (Default|ProneEvent _playercharacter)
    (else
      (Variables|Default|SetContadorEntrada 0)
      (Widget|RemovefromParent (stale OnComponentBeginOverlap(CollisionComponent) _returnvalue))
      (Utilities|FlowControl|Gate true) ; enters at Close
    )))

(event OnComponentBeginOverlap(CollisionComponent)
  (params (OverlappedComponent :type Primitive%20Component%20Object%20Reference) (OtherActor :type Actor%20Object%20Reference) (OtherComp :type Primitive%20Component%20Object%20Reference) (OtherBodyIndex :type Integer) (bFromSweep :type Boolean) (SweepResult :type Hit%20Result%20Structure%20%28by%20ref%29))
  (bind _playercharacter (Variables|Default|GetPlayerCharacter))
  (Utilities|Casting|CastToFirstPersonCharacter OtherActor)
  (Utilities|FlowControl|Sequence
    (:then_0
      (if (== (Variables|Default|GetContadorEntrada) 0)
        (Variables|Default|SetContadorEntrada 1)
        (bind _returnvalue (UserInterface|CreateWidget "/Game/Widgets/TutorialWidget/InstruccionesWidget.InstruccionesWidget_C"))
        (Variables|/Game/Widgets/TutorialWidget/InstruccionesWidget.InstruccionesWidget_C|SetTextoInstruccionesAlternativas _returnvalue "Pulsa \"E\" para esconderte bajo el coche")
        (UserInterface|Viewport|AddtoViewport _returnvalue 0)))
    (:then_1
      (Utilities|FlowControl|Gate true) ; enters at Open
    )))

(event Custom|Prone-Tumbado
  (bind _playercharacter (Variables|Default|GetPlayerCharacter))
  (Utilities|FlowControl|Gate true
    (:Exit
      (if (not (Variables|/Game/FirstPersonBP/Blueprints/FirstPersonCharacter.FirstPersonCharacter_C|GetProne (Variables|Default|GetPlayerCharacter)))
        (Variables|Default|SetContadorEntrada 0)
        (Widget|RemovefromParent (stale OnComponentBeginOverlap(CollisionComponent) _returnvalue))
        (Class|AIPerceptionStimuliSourceComponent|UnregisterfromSense (Variables|/Game/FirstPersonBP/Blueprints/FirstPersonCharacter.FirstPersonCharacter_C|GetAIPerceptionStimuliSource _playercharacter) "/Script/AIModule.AISense_Sight")
        (Default|ProneEvent _playercharacter)))))

(event Custom|MoveYaw
  (params (AxisVal :type Float%20%28single-precision%29)))

(event Custom|MovePitch
  (params (Axis%20Val :type Float%20%28single-precision%29))
  (bind _camerainside (Variables|Default|GetCameraInside))
  (bind _returnvalue (Transformation|GetActorRotation _camerainside))
  (if (and (>= (.pitch _returnvalue) -35.0) (<= (.pitch _returnvalue) 25.0))
    (Transformation|AddActorLocalRotation (Variables|Default|GetCameraInside) (Math|Rotator|MakeRotator 0.0 (* Axis%20Val -1.0) 0.0) false false :!label _label)
    (else
      ;[1 1 1] Comprobación de límite por abajo
      (if (and (< (.pitch _returnvalue) -35.0) (> 0.0 Axis%20Val))
        (goto _label)
        (else
          ;[1 1 1] Comprobación de límite por arriba
          (if (and (< 25.0 (.pitch _returnvalue)) (> Axis%20Val 0.0))
            (goto _label)))))))

(event EventBeginPlay
  (bind _asfirst_person_character (Utilities|Casting|CastToFirstPersonCharacter (Game|GetPlayerCharacter 0)))
  (Variables|Default|SetPlayerCharacter _asfirst_person_character))

(event Collision|EventActorBeginOverlap
  (params (OtherActor :type Actor%20Object%20Reference)))

(event EventTick
  (params (DeltaSeconds :type Float%20%28single-precision%29)))

(fn ConstructionScript)