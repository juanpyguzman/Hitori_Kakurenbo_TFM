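; Trigger box that marks the ground floor (planta baja), tracking whether the player or enemy has entered it.
; On overlap, a FirstPersonCharacter gets its first-floor flag cleared.
; A BP_Enemy_2 has the matching flag cleared on its AI controller instead.
; Each case prints a debug message naming who arrived.
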(event OnComponentBeginOverlap(CollisionComponent)
  (params (OverlappedComponent :type Primitive%20Component%20Object%20Reference) (OtherActor :type Actor%20Object%20Reference) (OtherComp :type Primitive%20Component%20Object%20Reference) (OtherBodyIndex :type Integer) (bFromSweep :type Boolean) (SweepResult :type Hit%20Result%20Structure%20%28by%20ref%29))
  (Utilities|FlowControl|Sequence
    (:then_0
      (bind _asfirst_person_character (Utilities|Casting|CastToFirstPersonCharacter OtherActor))
      (Variables|/Game/FirstPersonBP/Blueprints/FirstPersonCharacter.FirstPersonCharacter_C|SetPlayerEnPrimeraPlanta _asfirst_person_character false)
      (Development|PrintString (Utilities|String|Append "Niño en Planta Baja" "")))
    (:then_1
      (bind _asbp_enemy_2 (Utilities|Casting|CastToBP_Enemy_2 OtherActor))
      (bind _asbp_aicontroller_enemy_2 (Utilities|Casting|CastToBP_AIController_Enemy_2 (AI|GetAIController _asbp_enemy_2)))
      (Variables|/Game/Muñeco/IA/BP_AIController_Enemy_2.BP_AIController_Enemy_2_C|SetEnemyEnPrimeraPlanta _asbp_aicontroller_enemy_2 false)
      (Development|PrintString (Utilities|String|Append "Remiendos en Planta Baja" "") true true "(R=0.000000,G=0.660000,B=1.000000,A=1.000000)" 1e+01))))

(event EventBeginPlay)

(event Collision|EventActorBeginOverlap
  (params (OtherActor :type Actor%20Object%20Reference)))

(event EventTick
  (params (DeltaSeconds :type Float%20%28single-precision%29)))

(fn ConstructionScript)