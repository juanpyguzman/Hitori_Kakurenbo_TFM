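; Tutorial trigger box that shows the crouch instruction ("Right click to crouch") to the player once.
; When the FirstPersonCharacter begins overlapping and the GlobalVariables game instance has TutorialEncendido on, it creates an InstruccionesWidget, adds it to the viewport and sets its text.
; Leaving the box removes the widget, and the Contador state counter keeps the prompt from appearing again.
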(event OnComponentBeginOverlap(CollisionComponent)
  (params (OverlappedComponent :type Primitive%20Component%20Object%20Reference) (OtherActor :type Actor%20Object%20Reference) (OtherComp :type Primitive%20Component%20Object%20Reference) (OtherBodyIndex :type Integer) (bFromSweep :type Boolean) (SweepResult :type Hit%20Result%20Structure%20%28by%20ref%29))
  (bind _asglobal_variables (Utilities|Casting|CastToGlobalVariables (Game|GetGameInstance)))
  (if (Variables|/Game/FirstPersonBP/GlobalVariables.GlobalVariables_C|GetTutorialEncendido _asglobal_variables)
    (Utilities|Casting|CastToFirstPersonCharacter OtherActor)
    (if (== (Variables|Default|GetContador) 0)
      (bind _returnvalue (UserInterface|CreateWidget "/Game/Widgets/TutorialWidget/InstruccionesWidget.InstruccionesWidget_C"))
      (UserInterface|Viewport|AddtoViewport _returnvalue 0)
      (Variables|/Game/Widgets/TutorialWidget/InstruccionesWidget.InstruccionesWidget_C|SetTextoInstrucciones1 _returnvalue "Right click to crouch")
      (Variables|Default|SetContador 1))))

(event OnComponentEndOverlap(CollisionComponent)
  (params (OverlappedComponent :type Primitive%20Component%20Object%20Reference) (OtherActor :type Actor%20Object%20Reference) (OtherComp :type Primitive%20Component%20Object%20Reference) (OtherBodyIndex :type Integer))
  (if (== (Variables|Default|GetContador) 1)
    (Utilities|Casting|CastToFirstPersonCharacter OtherActor)
    (Widget|RemovefromParent (stale OnComponentBeginOverlap(CollisionComponent) _returnvalue))
    (Variables|Default|SetContador 2)))

(event EventBeginPlay)

(event Collision|EventActorBeginOverlap
  (params (OtherActor :type Actor%20Object%20Reference)))

(event EventTick
  (params (DeltaSeconds :type Float%20%28single-precision%29)))

(fn ConstructionScript)