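; Hatch to the upper floor that swings open when its AbrirTrampilla event is called, intended as a key-operated opening.
; A sphere trigger tracks whether the first-person character is nearby until the key is used, showing an instruction widget when the GameInstance tutorial flag is on.
; AbrirTrampilla removes that widget and plays a timeline that rotates the actor on roll.
; A PlaySound flag limits the key sound to one play and marks the key as used.
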(event OnComponentBeginOverlap(Sphere)
  (params (OverlappedComponent :type Primitive%20Component%20Object%20Reference) (OtherActor :type Actor%20Object%20Reference) (OtherComp :type Primitive%20Component%20Object%20Reference) (OtherBodyIndex :type Integer) (bFromSweep :type Boolean) (SweepResult :type Hit%20Result%20Structure%20%28by%20ref%29))
  (if (not (Variables|Default|GetLlaveUsada))
    (Utilities|Casting|CastToFirstPersonCharacter OtherActor)
    (Variables|Default|SetCharacterIsOverlapping true)
    (bind _asglobal_variables (Utilities|Casting|CastToGlobalVariables (Game|GetGameInstance)))
    (if (Variables|/Game/FirstPersonBP/GlobalVariables.GlobalVariables_C|GetTutorialEncendido _asglobal_variables)
      (if (== (Variables|Default|GetContador) 0)
        (Variables|Default|SetContador 1)
        (bind _returnvalue (UserInterface|CreateWidget "/Game/Widgets/TutorialWidget/InstruccionesWidget.InstruccionesWidget_C"))
        (Variables|/Game/Widgets/TutorialWidget/InstruccionesWidget.InstruccionesWidget_C|SetTextoInstruccionesAlternativas _returnvalue "Usa la llave para abrir la trampilla de acceso a la planta superior")
        (UserInterface|Viewport|AddtoViewport _returnvalue 0)))))

(event OnComponentEndOverlap(Sphere)
  (params (OverlappedComponent :type Primitive%20Component%20Object%20Reference) (OtherActor :type Actor%20Object%20Reference) (OtherComp :type Primitive%20Component%20Object%20Reference) (OtherBodyIndex :type Integer))
  (if (not (Variables|Default|GetLlaveUsada))
    (Utilities|Casting|CastToFirstPersonCharacter OtherActor)
    (Variables|Default|SetCharacterIsOverlapping false)
    (bind _asglobal_variables (Utilities|Casting|CastToGlobalVariables (Game|GetGameInstance)))
    (if (Variables|/Game/FirstPersonBP/GlobalVariables.GlobalVariables_C|GetTutorialEncendido _asglobal_variables)
      (Variables|Default|SetContador 0)
      (Widget|RemovefromParent (stale OnComponentBeginOverlap(Sphere) _returnvalue)))))

(event Custom|Abrir%20Trampilla
  (Widget|RemovefromParent (stale OnComponentBeginOverlap(Sphere) _returnvalue))
  (bind _angle (Timeline|Apertura%20de%20Trampilla Play)
    (:Update
      (Transformation|SetActorRelativeRotation (Math|Rotator|MakeRotator (* _angle -8e+01) 0.0 0.0))
      (if (Variables|Default|GetPlaySound)
        (Audio|PlaySoundatLocation "/Game/Widgets/HUD/Sounds/UseObjects/KeyOpeningHatch.KeyOpeningHatch" (Transformation|GetActorLocation self) "0, 0, 0" 1.0 1.0 0.0 0 0 0)
        (Variables|Default|SetPlaySound false)
        (Variables|Default|SetLlaveUsada true)))))

(event EventBeginPlay
  (Variables|Default|SetCharacterIsOverlapping false)
  (Variables|Default|SetLlaveUsada false))

(event Collision|EventActorBeginOverlap
  (params (OtherActor :type Actor%20Object%20Reference)))

(event EventTick
  (params (DeltaSeconds :type Float%20%28single-precision%29)))

(fn ConstructionScript)