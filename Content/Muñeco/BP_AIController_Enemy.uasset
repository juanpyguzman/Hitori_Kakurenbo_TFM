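; AI controller for an enemy that chases the player while the player is stopped and wanders otherwise.
; Tick reads PlayerIsStopped from FirstPersonCharacter and uses BB_Enemy bools to trigger Chasing or Wandering only on a state change.
; Each event sets TargetPoint once, near the player controller or randomly around the enemy, then runs BT_Enemy.
; Debug prints show a separately sampled random point, not the stored target.
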(event Custom|Chasing
  (bind _returnvalue (Game|GetPlayerController 0))
  (bind _returnvalue_2 (Transformation|GetActorLocation _returnvalue))
  (bind _randomlocation (AI|Navigation|GetRandomReachablePointinRadius _returnvalue_2 1e+01 0 0))
  ;[1 1 1] Chasing event
  (AI|Components|Blackboard|SetValueasBool (stale EventTick _blackboardcomponent) (Utilities|Name|MakeLiteralName "IsWandering") false)
  (AI|Components|Blackboard|SetValueasBool (stale EventTick _blackboardcomponent) (Utilities|Name|MakeLiteralName "IsChasing") true)
  (AI|Components|Blackboard|SetValueasVector (stale EventTick _blackboardcomponent) (Utilities|Name|MakeLiteralName "TargetPoint") _randomlocation)
  (AI|RunBehaviorTree "/Game/Muñeco/BT_Enemy.BT_Enemy")
  (Development|PrintString (Utilities|String|ToString(Vector) _randomlocation) true true "(R=1.000000,G=0.000000,B=0.085713,A=1.000000)" 1e+01)
  (AI|Components|Blackboard|SetValueasBool (stale EventTick _blackboardcomponent) (Utilities|Name|MakeLiteralName "IsWandering") false)
  (AI|Components|Blackboard|SetValueasBool (stale EventTick _blackboardcomponent) (Utilities|Name|MakeLiteralName "IsChasing") true))

(event Custom|Wandering
  (bind _returnvalue (Pawn|GetControlledPawn))
  (bind _returnvalue_2 (Transformation|GetActorLocation _returnvalue))
  (bind _randomlocation (AI|Navigation|GetRandomReachablePointinRadius _returnvalue_2 1e+04 0 0))
  ;[1 1 1] Wandering event
  (AI|Components|Blackboard|SetValueasBool (stale EventTick _blackboardcomponent) (Utilities|Name|MakeLiteralName "IsWandering") true)
  (AI|Components|Blackboard|SetValueasBool (stale EventTick _blackboardcomponent) (Utilities|Name|MakeLiteralName "IsChasing") false)
  (AI|Components|Blackboard|SetValueasVector (stale EventTick _blackboardcomponent) (Utilities|Name|MakeLiteralName "TargetPoint") _randomlocation)
  (AI|RunBehaviorTree "/Game/Muñeco/BT_Enemy.BT_Enemy")
  (Development|PrintString (Utilities|String|ToString(Vector) _randomlocation) true true "(R=0.000000,G=0.660000,B=1.000000,A=1.000000)" 1e+01)
  (AI|Components|Blackboard|SetValueasBool (stale EventTick _blackboardcomponent) (Utilities|Name|MakeLiteralName "IsWandering") true)
  (AI|Components|Blackboard|SetValueasBool (stale EventTick _blackboardcomponent) (Utilities|Name|MakeLiteralName "IsChasing") false))

(event EventBeginPlay
  (bind _blackboardcomponent (Class|AIController|UseBlackboard "/Game/Muñeco/BB_Enemy.BB_Enemy"))
  (AI|Components|Blackboard|SetValueasBool _blackboardcomponent (Utilities|Name|MakeLiteralName "IsWandering") false)
  (AI|Components|Blackboard|SetValueasBool _blackboardcomponent (Utilities|Name|MakeLiteralName "IsChasing") false))

(event EventTick
  (params (DeltaSeconds :type Float%20%28single-precision%29))
  (bind _blackboardcomponent (Class|AIController|UseBlackboard "/Game/Muñeco/BB_Enemy.BB_Enemy"))
  (bind _asfirst_person_character (Utilities|Casting|CastToFirstPersonCharacter (Game|GetPlayerCharacter 0)))
  (if (Variables|/Game/FirstPersonBP/Blueprints/FirstPersonCharacter.FirstPersonCharacter_C|GetPlayerIsStopped _asfirst_person_character)
    (if (not (ScalableFloat|GetValueasBool _blackboardcomponent (Utilities|Name|MakeLiteralName "IsChasing")))
      (CallFunction|Chasing))
    (elif (not (ScalableFloat|GetValueasBool _blackboardcomponent (Utilities|Name|MakeLiteralName "IsWandering")))
      (CallFunction|Wandering))))

(fn ConstructionScript)