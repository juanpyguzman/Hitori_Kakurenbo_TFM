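; BP_Enemy_2 is the Remiendos enemy, whose perception feeds state flags on its BP_AIController_Enemy_2.
; On BeginPlay it reads the tutorial flag from the GlobalVariables game instance, teleports to the tutorial or normal start, and informs the controller.
; Perceiving the player sets IsSeeing, while TimerAlarm stimuli set IsHearingSound, then clear it after the alarm sound's duration.
; A custom event plays its footstep audio.
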(event OnTargetPerceptionUpdated(AIPerception)
  (params (Actor :type Actor%20Object%20Reference) (Stimulus :type AI%20Stimulus%20Structure))
  (bind _asfirst_person_character (Utilities|Casting|CastToFirstPersonCharacter Actor)
    (:then
      (Development|PrintString (Utilities|String|Append (Utilities|GetDisplayName _asfirst_person_character) (Utilities|String|ToString(Boolean) (.bsuccessfullysensed Stimulus))))
      (bind _asbp_aicontroller_enemy_2 (Utilities|Casting|CastToBP_AIController_Enemy_2 (AI|GetAIController self)))
      (Variables|/Game/Muñeco/IA/BP_AIController_Enemy_2.BP_AIController_Enemy_2_C|SetIsSeeing _asbp_aicontroller_enemy_2 (.bsuccessfullysensed Stimulus)))
    (:CastFailed
      (if (Utilities|Name|Equal(Name) (.tag Stimulus) "TimerAlarm")
        (bind _asbp_aicontroller_enemy_2_2 (Utilities|Casting|CastToBP_AIController_Enemy_2 (AI|GetAIController self)))
        (Variables|/Game/Muñeco/IA/BP_AIController_Enemy_2.BP_AIController_Enemy_2_C|SetIsHearingSound _asbp_aicontroller_enemy_2_2 (.bsuccessfullysensed Stimulus))
        (bind _asglobal_variables (Utilities|Casting|CastToGlobalVariables (Game|GetGameInstance)))
        (Utilities|FlowControl|Delay (Variables|/Script/Engine.SoundBase|GetDuration (Variables|/Script/Engine.AudioComponent|GetSound (Variables|/Game/FirstPersonBP/GlobalVariables.GlobalVariables_C|GetAudioTimerAlarm _asglobal_variables))))
        (Variables|/Game/Muñeco/IA/BP_AIController_Enemy_2.BP_AIController_Enemy_2_C|SetIsHearingSound _asbp_aicontroller_enemy_2_2 false)))))

(event Custom|EventoPisadasRemiendos
  (Audio|Components|Audio|Play (Variables|Default|GetRemiendosFootsteps) 0.0))

(event EventBeginPlay
  (bind _asglobal_variables (Utilities|Casting|CastToGlobalVariables (Game|GetGameInstance)))
  (if (Variables|/Game/FirstPersonBP/GlobalVariables.GlobalVariables_C|GetTutorialEncendido _asglobal_variables)
    (Transformation|SetActorLocation "2496.824707,1313.992065,1012.846619" false false)
    (bind _asbp_aicontroller_enemy_2 (Utilities|Casting|CastToBP_AIController_Enemy_2 (AI|GetAIController self)))
    (Variables|/Game/Muñeco/IA/BP_AIController_Enemy_2.BP_AIController_Enemy_2_C|SetTutorial _asbp_aicontroller_enemy_2 true)
    (else
      (Transformation|SetActorLocation (Variables|Default|GetRemiendosStartPosition) false false)
      (bind _asbp_aicontroller_enemy_2_2 (Utilities|Casting|CastToBP_AIController_Enemy_2 (AI|GetAIController self)))
      (Variables|/Game/Muñeco/IA/BP_AIController_Enemy_2.BP_AIController_Enemy_2_C|SetTutorial _asbp_aicontroller_enemy_2_2 false))))

(fn ConstructionScript)