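; AI controller for the second enemy type, which runs its behavior tree and feeds its blackboard every tick.
; The player's stopped and moving states drive the going-to-zone, wandering and movement flags.
; It raises an alert when the enemy's navigation path to the bathroom exceeds the player's by a threshold.
; While IsSeeing is true, a short path to the player sets the attacking flag; sight and position values are not updated here.
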(event EventBeginPlay
  (Variables|Default|SetIsSeeing false)
  (AI|RunBehaviorTree "/Game/Muñeco/IA/BT_Enemy_2.BT_Enemy_2"))

(event EventTick
  (params (DeltaSeconds :type Float%20%28single-precision%29))
  (bind _isseeing (Variables|Default|GetIsSeeing))
  (bind _asfirst_person_character (Utilities|Casting|CastToFirstPersonCharacter (Game|GetPlayerCharacter 0)))
  (bind _blackboardcomponent (Class|AIController|UseBlackboard "/Game/Muñeco/IA/BB_Enemy_2.BB_Enemy_2"))
  (AI|Components|Blackboard|SetValueasBool _blackboardcomponent (Utilities|Name|MakeLiteralName "IsGoingToZone") (Variables|/Game/FirstPersonBP/Blueprints/FirstPersonCharacter.FirstPersonCharacter_C|GetPlayerIsStopped _asfirst_person_character))
  (AI|Components|Blackboard|SetValueasBool _blackboardcomponent (Utilities|Name|MakeLiteralName "IsWandering") (not (Variables|/Game/FirstPersonBP/Blueprints/FirstPersonCharacter.FirstPersonCharacter_C|GetPlayerIsStopped _asfirst_person_character)))
  (AI|Components|Blackboard|SetValueasBool _blackboardcomponent (Utilities|Name|MakeLiteralName "PlayerIsMoving") (Variables|/Game/FirstPersonBP/Blueprints/FirstPersonCharacter.FirstPersonCharacter_C|GetPlayerIsMoving _asfirst_person_character))
  (Variables|Default|SetEnemyDistanceToBath (.PathLength (Class|NavigationSystemV1|GetPathLength (Variables|Default|GetEnemyPosition) (Variables|Default|GetBathroomPointPosition) 0 0)))
  (Variables|Default|SetPlayerDistanceToBath (.PathLength (Class|NavigationSystemV1|GetPathLength (Variables|Default|GetPlayerPosition) (Variables|Default|GetBathroomPointPosition) 0 0)))
  (Utilities|FlowControl|Sequence
    (:then_0
      (if (> (- (Variables|Default|GetEnemyDistanceToBath) (Variables|Default|GetPlayerDistanceToBath)) (Variables|Default|GetDistanciaMínimaAlerta))
        (bind _output_get (Variables|Default|SetIsAlerted true))
        (AI|Components|Blackboard|SetValueasBool _blackboardcomponent (Utilities|Name|MakeLiteralName "IsAlerted") _output_get)
        (else
          (bind _output_get_2 (Variables|Default|SetIsAlerted false))
          (AI|Components|Blackboard|SetValueasBool _blackboardcomponent (Utilities|Name|MakeLiteralName "IsAlerted") _output_get_2))))
    (:then_1
      (AI|Components|Blackboard|SetValueasBool _blackboardcomponent (Utilities|Name|MakeLiteralName "IsSeeing") _isseeing)
      (if _isseeing
        (bind _output_get_3 (Variables|Default|SetEnemyPlayerDistance (.PathLength (Class|NavigationSystemV1|GetPathLength (Variables|Default|GetEnemyPosition) (Variables|Default|GetPlayerPosition) 0 0))))
        (if (< _output_get_3 2e+02)
          (bind _output_get_4 (Variables|Default|SetIsAttacking true))
          (AI|Components|Blackboard|SetValueasBool _blackboardcomponent (Utilities|Name|MakeLiteralName "IsAttacking") _output_get_4)
          (Development|PrintString "¡Ataque!" true true "(R=1.000000,G=0.043050,B=0.000000,A=1.000000)")
          (else
            (bind _output_get_5 (Variables|Default|SetIsAttacking false))
            (AI|Components|Blackboard|SetValueasBool _blackboardcomponent (Utilities|Name|MakeLiteralName "IsAttacking") _output_get_5)))))))

(fn ConstructionScript)